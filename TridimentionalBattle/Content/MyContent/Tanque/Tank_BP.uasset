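; Player-controlled tank Blueprint that wires input to driving, camera orbit and firing.
; On BeginPlay it hands barrel and turret to TankAiming and both tracks to TankMovement, which receive the fire and drive inputs.
; Look axes split yaw onto GiroscopoHorizontal and pitch onto SpringArm, avoiding combined rotation on one component.
; The R key zeroes the actor's rotation.
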(event EventBeginPlay
  (Class|TankAimingComponent|Iniciar (Variables|Default|GetTankAiming) (Variables|Default|GetBarrel) (Variables|Default|GetTurret))
  (Class|TankMovementComponent|Iniciar (Variables|Default|GetTankMovement) (Variables|Default|GetR_Track) (Variables|Default|GetL_Track)))

(event Input|KeyboardEvents|R
  (params (Key :type Key%20Structure))
  (:Pressed
    (Transformation|SetActorRotation "0, 0, 0")))

(event Input|ActionEvents|InputActionFire
  (params (Key :type Key%20Structure))
  (:Pressed
    (Class|TankAimingComponent|Fire (Variables|Default|GetTankAiming))))

(event Input|AxisEvents|InputAxisLookRight
  (params (AxisValue :type Float%20%28single-precision%29))
  ;[1 1 1] Input Setup
  (Transformation|AddLocalRotation (Variables|Default|GetGiroscopo%20Horizontal) (Math|Rotator|MakeRotator 0.0 0.0 AxisValue) false false))

(event Input|AxisEvents|InputAxisLookUp
  (params (AxisValue :type Float%20%28single-precision%29))
  ;[1 1 1] Input Setup
  (Transformation|AddLocalRotation (Variables|Default|GetSpringArm) (Math|Rotator|MakeRotator 0.0 AxisValue 0.0) false false))

(event Input|AxisEvents|InputAxisTurnRight
  (params (AxisValue :type Float%20%28single-precision%29))
  ;[1 1 1] Input Setup
  (Class|TankMovementComponent|IntendTurnRight (Variables|Default|GetTankMovement) AxisValue))

(event Input|AxisEvents|InputAxisForwardMovement
  (params (AxisValue :type Float%20%28single-precision%29))
  ;[1 1 1] Input Setup
  (Class|TankMovementComponent|IntendMovementForward (Variables|Default|GetTankMovement) AxisValue))

(fn ConstructionScript)